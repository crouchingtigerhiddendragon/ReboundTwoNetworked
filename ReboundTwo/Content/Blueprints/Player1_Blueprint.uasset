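; Player 1 pawn Blueprint that turns its static mesh left and right within a limited yaw arc.
; Two input axes drive the yaw, with the InFront flag choosing which one applies and SpeedDivider scaling the turn rate.
; Tick snaps the yaw back just inside fixed limits at either end.
; Tick also toggles the Sunnies component's visibility from an EasterEgg flag.
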(event EventTick
  (params (DeltaSeconds :type Float%20%28single-precision%29))
  (bind _staticmeshcomponent (Variables|Debug|GetStaticMeshComponent))
  (bind _sunnies (Variables|Default|Getsunnies))
  (bind _staticmeshcomponent_2 (Variables|Debug|GetStaticMeshComponent))
  ;[1 1 1] Curb Rotation
  (if (Variables|Default|GetEasterEgg)
    (Rendering|SetVisibility _sunnies true false)
    (else
      (Rendering|SetVisibility _sunnies false false)))
  (if (>= (.yaw (Transformation|GetWorldRotation _staticmeshcomponent_2)) 27.0)
    (Transformation|SetWorldRotation _staticmeshcomponent_2 (Math|Rotator|MakeRotator 0.0 0.0 26.8) false false)
    (elif (<= (.yaw (Transformation|GetWorldRotation _staticmeshcomponent)) -148.0)
      (Transformation|SetWorldRotation _staticmeshcomponent (Math|Rotator|MakeRotator 0.0 0.0 -147.8) false false))))

(event Input|AxisEvents|InputAxisP1Move
  (params (AxisValue :type Float%20%28single-precision%29))
  (bind _staticmeshcomponent (Variables|Debug|GetStaticMeshComponent))
  (bind _returnvalue (Transformation|GetWorldRotation _staticmeshcomponent))
  ;[1 1 1] Player Rotation Movement
  (if (Variables|Default|GetInFront)
    (Transformation|SetWorldRotation _staticmeshcomponent (Math|Rotator|MakeRotator (.roll _returnvalue) (.pitch _returnvalue) (+ (.yaw _returnvalue) (/ AxisValue (Variables|Default|GetSpeedDivider)))) false false)))

(event Input|AxisEvents|InputAxisAltP1Move
  (params (AxisValue :type Float%20%28single-precision%29))
  (bind _staticmeshcomponent (Variables|Debug|GetStaticMeshComponent))
  (bind _returnvalue (Transformation|GetWorldRotation _staticmeshcomponent))
  ;[1 1 1] Player Rotation Movement
  (if (not (Variables|Default|GetInFront))
    (Transformation|SetWorldRotation _staticmeshcomponent (Math|Rotator|MakeRotator (.roll _returnvalue) (.pitch _returnvalue) (+ (.yaw _returnvalue) (/ AxisValue (Variables|Default|GetSpeedDivider)))) false false)))

(fn ConstructionScript)