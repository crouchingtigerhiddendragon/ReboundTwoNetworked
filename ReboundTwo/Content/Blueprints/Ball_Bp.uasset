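; Pong ball actor that BallStart launches along X or Y at an initial speed, on authority only.
; Each Tick applies a velocity-cross-spin force to curve its flight, then clamps one out-of-range X or Y velocity component to MaxSpeed.
; Hit logic for blocks, paddles, goals, scoring and countdown respawn is disconnected, as is SetCamera's front-player swap, so neither runs.
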(event OnComponentHit(StaticMeshComponent)
  (params (HitComponent :type Primitive%20Component%20Object%20Reference) (OtherActor :type Actor%20Object%20Reference) (OtherComp :type Primitive%20Component%20Object%20Reference) (NormalImpulse :type Vector :default "0, 0, 0") (Hit :type Hit%20Result%20Structure%20%28by%20ref%29))
  ;[1 1 1] We love spaghetti in Blueprints <3
)

(event Custom|InitBall
  ;[1 1 1] Ball Initializes and Updates on server
  (CallFunction|BallStart))

(event Custom|UpdateBall
  (bind _staticmeshcomponent (Variables|Debug|GetStaticMeshComponent))
  (bind _staticmeshcomponent_2 (Variables|Debug|GetStaticMeshComponent))
  (bind _maxspeed (Variables|Default|GetMaxSpeed))
  (bind _maxspeed_2 (Variables|Default|GetMaxSpeed))
  (bind _returnvalue (* _maxspeed -1.0))
  (bind _returnvalue_2 (* _maxspeed_2 -1.0))
  ;[1 1 1] Ball Initializes and Updates on server
  (bind _returnvalue_3 (Physics|GetPhysicsLinearVelocity _staticmeshcomponent_2 "None"))
  (bind _returnvalue_4 (Class|PrimitiveComponent|GetPhysicsAngularVelocity _staticmeshcomponent_2 "None"))
  (Physics|AddForce _staticmeshcomponent_2 (* (Math|Vector|CrossProduct _returnvalue_3 _returnvalue_4) (Variables|Default|Getcurve%20strength)) "None" false)
  (bind _returnvalue_5 (Physics|GetPhysicsLinearVelocity (Variables|Debug|GetStaticMeshComponent) "None"))
  (if (> (.x _returnvalue_5) _maxspeed)
    (Physics|SetPhysicsLinearVelocity _staticmeshcomponent (Math|Vector|MakeVector _maxspeed_2 0.0 0.0) false "None")
    (elif (> (.y _returnvalue_5) _maxspeed)
      (Physics|SetPhysicsLinearVelocity _staticmeshcomponent (Math|Vector|MakeVector 0.0 _maxspeed_2 0.0) false "None")
      (elif (< (.x _returnvalue_5) _returnvalue)
        (Physics|SetPhysicsLinearVelocity _staticmeshcomponent (Math|Vector|MakeVector _returnvalue_2 0.0 0.0) false "None")
        (elif (< (.y _returnvalue_5) _returnvalue)
          (Physics|SetPhysicsLinearVelocity _staticmeshcomponent (Math|Vector|MakeVector 0.0 _returnvalue_2 0.0) false "None"))))))

(event EventBeginPlay
  ;[1 1 1] Ball Initializes and Updates on server
  (CallFunction|InitBall))

(event EventTick
  (params (DeltaSeconds :type Float%20%28single-precision%29))
  ;[1 1 1] Ball Initializes and Updates on server
  (CallFunction|UpdateBall))

(fn ConstructionScript)

(fn SetCamera)

(fn BallStart
  (bind _initialballspeed (Variables|Default|GetinitialBallSpeed))
  (bind _staticmeshcomponent (Variables|Debug|GetStaticMeshComponent))
  (Networking|SwitchHasAuthority
    (:Authority
      (if (Variables|Default|GetBallStartAtY%20%28if%20False%20Goes%20On%20X%20Axis%29)
        (Physics|SetPhysicsLinearVelocity _staticmeshcomponent (Math|Vector|MakeVector 0.0 _initialballspeed 0.0) false "None")
        (else
          (Physics|SetPhysicsLinearVelocity _staticmeshcomponent (Math|Vector|MakeVector _initialballspeed 0.0 0.0) false "None"))))))