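; Player 2 Blueprint that turns its static mesh around the yaw axis from player input and shows sunglasses when an EasterEgg flag is set.
; The InFront flag selects whether the P2Move or AltP2Move axis applies, with input scaled down by a speed divider.
; Tick bounds the rotation by snapping yaw back whenever it enters either of two narrow angle bands, acting as soft stops.
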(event EventTick
  (params (DeltaSeconds :type Float%20%28single-precision%29))
  (bind _staticmeshcomponent (Variables|Debug|GetStaticMeshComponent))
  (bind _staticmeshcomponent_2 (Variables|Debug|GetStaticMeshComponent))
  (bind _returnvalue (Transformation|GetWorldRotation _staticmeshcomponent))
  (bind _returnvalue_2 (Transformation|GetWorldRotation _staticmeshcomponent_2))
  (if (Variables|Default|GetEasterEgg)
    (Rendering|SetVisibility (Variables|Default|Getsunnies) true false)
    (else
      (Rendering|SetVisibility (Variables|Default|Getsunnies) false false)))
  (if (and (<= (.yaw _returnvalue_2) 2e+01) (>= (.yaw _returnvalue_2) 19.0))
    (Transformation|SetWorldRotation _staticmeshcomponent_2 (Math|Rotator|MakeRotator 0.0 0.0 21.8) false false)
    (elif (and (>= (.yaw _returnvalue) -137.0) (<= (.yaw _returnvalue) -136.0))
      (Transformation|SetWorldRotation _staticmeshcomponent (Math|Rotator|MakeRotator 0.0 0.0 -138.8) false false))))

(event Input|AxisEvents|InputAxisP2Move
  (params (AxisValue :type Float%20%28single-precision%29))
  (bind _staticmeshcomponent (Variables|Debug|GetStaticMeshComponent))
  (bind _returnvalue (Transformation|GetWorldRotation _staticmeshcomponent))
  (if (not (Variables|Default|GetInFront))
    (Transformation|SetWorldRotation _staticmeshcomponent (Math|Rotator|MakeRotator (.roll _returnvalue) (.pitch _returnvalue) (+ (.yaw _returnvalue) (/ AxisValue (Variables|Default|GetSpeedDevider)))) false false)))

(event Input|AxisEvents|InputAxisAltP2Move
  (params (AxisValue :type Float%20%28single-precision%29))
  (bind _staticmeshcomponent (Variables|Debug|GetStaticMeshComponent))
  (bind _returnvalue (Transformation|GetWorldRotation _staticmeshcomponent))
  (if (Variables|Default|GetInFront)
    (Transformation|SetWorldRotation _staticmeshcomponent (Math|Rotator|MakeRotator (.roll _returnvalue) (.pitch _returnvalue) (+ (.yaw _returnvalue) (/ AxisValue (Variables|Default|GetSpeedDevider)))) false false)))

(fn ConstructionScript)